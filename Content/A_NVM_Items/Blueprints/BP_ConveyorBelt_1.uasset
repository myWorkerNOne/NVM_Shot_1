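; Spline-shaped conveyor belt that carries overlapping actors along its path at DynamicSpeed.
; The construction script builds two spline meshes per segment: a visible one with length-scaled material and another for overlap detection.
; A fast looping timer offsets each overlapping actor once per tick along the nearest spline direction, sweeping only Characters.
; The BeltLooper timeline, meant to animate the material's PTime, has nothing triggering it in the graph.
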(event `self.ReceiveBeginPlay`
  (`KismetSystemLibrary.K2_SetTimerDelegate` (delegate `Move Objects`) 0.01 true))

(event `Move Objects`
  (set `self.MoveActors` (`|MakeArray` self :!type "Actor Object Reference"))
  (for _array_element (`self.OverlapComponents`)
    (for _array_element_2 (`PrimitiveComponent.GetOverlappingActors` _array_element null)
      (if (== (`KismetArrayLibrary.Array_Find` (`self.MoveActors`) _array_element_2) -1)
        (cast `Character` _array_element_2
          (:`then`
            (bind _returnvalue (`KismetMathLibrary.GreaterGreater_VectorRotator` (* (`SplineComponent.FindDirectionClosestToWorldLocation` (`self.Spline`) (`self.K2_GetActorLocation` _array_element_2) "Local") (`self.DynamicSpeed`)) (`SceneComponent.K2_GetComponentRotation` (`self.DefaultSceneRoot`))))
            (`self.K2_AddActorWorldOffset` _array_element_2 _returnvalue true false))
          (:`CastFailed`
            (`self.K2_AddActorWorldOffset` _array_element_2 _returnvalue false false)))
        (`KismetArrayLibrary.Array_Add` (`self.MoveActors`) _array_element_2)))))

(fn `UserConstructionScript`
  (bind _spline (`self.Spline`))
  (bind _spline_2 (`self.Spline`))
  (for _index (range (+ (- (`SplineComponent.GetNumberOfSplinePoints` (`self.Spline`)) 2) 1))
    (bind _returnvalue (`AddComponent|NODE_AddSplineMeshComponent-0`))
    (`KismetArrayLibrary.Array_Add` (`self.MeshComponents`) _returnvalue)
    (bind (_location _tangent) (`SplineComponent.GetLocationAndTangentAtSplinePoint` _spline_2 _index "Local"))
    (bind _returnvalue_2 (- _index -1))
    (bind (_location_2 _tangent_2) (`SplineComponent.GetLocationAndTangentAtSplinePoint` _spline_2 _returnvalue_2 "Local"))
    (`SplineMeshComponent.SetStartAndEnd` _returnvalue _location _tangent _location_2 _tangent_2 true)
    (`MeshComponent.SetScalarParameterValueOnMaterials` _returnvalue "XScale" (/ (- (`SplineComponent.GetDistanceAlongSplineAtSplinePoint` _spline _returnvalue_2) (`SplineComponent.GetDistanceAlongSplineAtSplinePoint` _spline _index)) 100.0))
    (bind _returnvalue_3 (`AddComponent|NODE_AddSplineMeshComponent-1`))
    (`KismetArrayLibrary.Array_Add` (`self.OverlapComponents`) _returnvalue_3)
    (`SplineMeshComponent.SetStartAndEnd` _returnvalue_3 _location _tangent _location_2 _tangent_2 true)))